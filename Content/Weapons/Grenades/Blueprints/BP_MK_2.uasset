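; BP_MK_2 is an MK 2 grenade actor that plays a pin-pull, throw and explosion sequence when the 2 key is pressed.
; Timed skeletal animations hide the pin and lever bones, then a timeline moves the mesh along a location track.
; Its update chain spawns a lever actor at a socket, fires delayed explosion particles and sound at world origin, then moves the mesh again and unhides both bones.
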(event EventBeginPlay
  ;[1 1 1] Player Input
  (Input|EnableInput (Game|GetPlayerController 0)))

(event Input|KeyboardEvents|2
  (params (Key :type Key%20Structure))
  (bind _mk_2_skeletal (Variables|Default|GetMK_2_Skeletal))
  (bind _mk_2_skeletal_2 (Variables|Default|GetMK_2_Skeletal))
  (bind _mk_2_skeletal_3 (Variables|Default|GetMK_2_Skeletal))
  (:Pressed
    ;[1 1 1] Safety_Pin_Remove
    (Components|Animation|PlayAnimation _mk_2_skeletal_3 "/Game/Weapons/Grenades/Animations/AS_MK_2_Safety_Pin_Remove.AS_MK_2_Safety_Pin_Remove" false)
    (Utilities|FlowControl|Delay 0.85)
    (Components|SkinnedMesh|HideBonebyName _mk_2_skeletal_3 "Safety_Pin" "PBO_None")
    (Utilities|FlowControl|Delay 0.3)
    ;[1 1 1] Release
    (Components|Animation|PlayAnimation _mk_2_skeletal_2 "/Game/Weapons/Grenades/Animations/AS_MK_2_Release.AS_MK_2_Release" false)
    (Utilities|FlowControl|Delay 0.1)
    (Components|SkinnedMesh|HideBonebyName _mk_2_skeletal_2 "Safety_Lever" "PBO_None")
    ;[1 1 1] Throw
    (bind _newtrack_0 (Timeline|Timeline_0 PlayFromStart)
      (:Update
        (Components|MoveComponentTo (Variables|Default|GetMK_2_Skeletal) _newtrack_0 "0, 0, 0" false false 0.2 false)
        ;[1 1 1] Lever Ejector
        (Game|SpawnActorfromClass "/Game/Weapons/Grenades/Blueprints/BP_MK_2_Lever.BP_MK_2_Lever_C" (Transformation|GetWorldTransform (Variables|Default|GetLever_Socket)) "Undefined" 0 0)
        ;[1 1 1] Explosion
        (Utilities|FlowControl|Delay 1.0)
        (Components|Activation|Activate (Variables|Default|GetPS_MK_2_Explosion) true)
        (Audio|SpawnSoundatLocation "/Game/Weapons/Grenades/Sounds/Cue/S_MK_2_Explosion_Cue.S_MK_2_Explosion_Cue" "0, 0, 0" "0, 0, 0" 1.0 1.0 0.0 0 0)
        ;[1 1 1] Respawn
        (Utilities|FlowControl|Delay 2.0)
        (Components|MoveComponentTo (Variables|Default|GetMK_2_Skeletal) "0, 0, 0" "0, 0, 0" false false 0.0 false)
        (Components|SkinnedMesh|UnHideBonebyName _mk_2_skeletal "Safety_Lever")
        (Components|SkinnedMesh|UnHideBonebyName _mk_2_skeletal "Safety_Pin")))))

(fn ConstructionScript)