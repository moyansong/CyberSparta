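; BP_M_18_Green is an M-18 green smoke grenade actor that plays a scripted pin-pull, release and throw when 7 is pressed.
; Delays sequence skeletal animations, bone hiding for pin and lever, a spawned lever actor, initial smoke and a fixed-location sound.
; A timeline then drives the mesh along the throw, triggers larger smoke, and later resets the mesh's position and hidden bones.
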(event EventBeginPlay
  ;[1 1 1] Player Input
  (Input|EnableInput (Game|GetPlayerController 0)))

(event Input|KeyboardEvents|7
  (params (Key :type Key%20Structure))
  (bind _m_18_green_skeletal (Variables|Default|GetM_18_Green_Skeletal))
  (bind _m_18_green_skeletal_2 (Variables|Default|GetM_18_Green_Skeletal))
  (bind _m_18_green_skeletal_3 (Variables|Default|GetM_18_Green_Skeletal))
  (:Pressed
    ;[1 1 1] Safety_Pin_Remove
    (Components|Animation|PlayAnimation _m_18_green_skeletal_3 "/Game/Weapons/Grenades/Animations/AS_M_18_Safety_Pin_Remove.AS_M_18_Safety_Pin_Remove" false)
    (Utilities|FlowControl|Delay 0.85)
    (Components|SkinnedMesh|HideBonebyName _m_18_green_skeletal_3 "Safety_Pin" "PBO_None")
    (Utilities|FlowControl|Delay 0.3)
    ;[1 1 1] Release
    (Components|Animation|PlayAnimation _m_18_green_skeletal_2 "/Game/Weapons/Grenades/Animations/AS_M_18_Release.AS_M_18_Release" false)
    (Utilities|FlowControl|Delay 0.1)
    (Components|SkinnedMesh|HideBonebyName _m_18_green_skeletal_2 "Safety_Lever" "PBO_None")
    ;[1 1 1] Lever Ejector
    (Game|SpawnActorfromClass "/Game/Weapons/Grenades/Blueprints/BP_M_18_Lever.BP_M_18_Lever_C" (Transformation|GetWorldTransform (Variables|Default|GetLever_Socket)) "Undefined" 0 0)
    ;[1 1 1] Start_Smoke
    (Components|Activation|Activate (Variables|Default|GetPS_M_18_Smoke_1) false)
    (Audio|SpawnSoundatLocation "/Game/Weapons/Grenades/Sounds/Cue/S_Smoke_Release_Cue.S_Smoke_Release_Cue" "-2099.048584,-800.000000,193.550858" "0, 0, 0" 1.0 1.0 0.0 0 0)
    (Utilities|FlowControl|Delay 1.0)
    ;[1 1 1] Throw
    (bind _newtrack_0 (Timeline|Timeline_0 Play)
      (:Update
        (Components|MoveComponentTo (Variables|Default|GetM_18_Green_Skeletal) _newtrack_0 "0, 0, 0" false false 0.2 false)
        ;[1 1 1] Big_Smoke_Release
        (Utilities|FlowControl|Delay 1.0)
        (Components|Activation|Activate (Variables|Default|GetPS_M_18_Smoke_2) true)
        ;[1 1 1] Respawn
        (Utilities|FlowControl|Delay 1e+01)
        (Components|MoveComponentTo _m_18_green_skeletal "0, 0, 0" "0, 0, 0" false false 0.0 false)
        (Components|SkinnedMesh|UnHideBonebyName _m_18_green_skeletal "Safety_Lever")
        (Components|SkinnedMesh|UnHideBonebyName _m_18_green_skeletal "Safety_Pin")))))

(fn ConstructionScript)